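; Enemy_Looking is a Paper2D enemy that watches for the player's blob and flips its facing every five seconds.
; Between flips, Tick alternates through a looping MultiGate: attacking inside the Killbox destroys it, while an unhidden player in the DetectionBox makes it launch along its yaw sign.
; ShotBP hits reduce its HP until destruction.
; Touching its Box knocks back and damages an unhidden blob.
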(event OnComponentBeginOverlap(PaperSprite)
  (params (OverlappedComponent :type Primitive%20Component%20Object%20Reference) (OtherActor :type Actor%20Object%20Reference) (OtherComp :type Primitive%20Component%20Object%20Reference) (OtherBodyIndex :type Integer) (bFromSweep :type Boolean) (SweepResult :type Hit%20Result%20Structure%20%28by%20ref%29))
  (bind _asshot_bp (Utilities|Casting|CastToShotBP OtherActor))
  (Actor|DestroyActor _asshot_bp)
  (Variables|Default|SetEnemyHP (- (Variables|Default|GetEnemyHP) 1))
  (if (<= (Variables|Default|GetEnemyHP) 0)
    (Actor|DestroyActor)))

(event OnComponentBeginOverlap(Box)
  (params (OverlappedComponent :type Primitive%20Component%20Object%20Reference) (OtherActor :type Actor%20Object%20Reference) (OtherComp :type Primitive%20Component%20Object%20Reference) (OtherBodyIndex :type Integer) (bFromSweep :type Boolean) (SweepResult :type Hit%20Result%20Structure%20%28by%20ref%29))
  (bind _asblob_bp (Utilities|Casting|CastToBlobBP OtherActor))
  (if (not (Variables|/Game/Blob/Blueprint/BlobBP.BlobBP_C|GetIsHiding _asblob_bp))
    (Character|LaunchCharacter _asblob_bp (Math|Vector|MakeVector (* (.x (.Normal (Collision|BreakHitResult SweepResult))) -4.5e+02) 0.0 4e+02) true true)
    (Default|DamageSystem _asblob_bp (Variables|Default|GetDamage))))

(event EventTick
  (params (DeltaSeconds :type Float%20%28single-precision%29))
  (bind _output_get (Variables|Default|SetSeconds (+ DeltaSeconds (Variables|Default|GetSeconds))))
  (if (< _output_get 5.0)
    (bind _asblob_bp (Utilities|Casting|CastToBlobBP (Game|GetPlayerCharacter 0)))
    (Utilities|FlowControl|MultiGate false true -1
      (:Out%200
        (if (Collision|IsOverlappingActor (Variables|Default|GetKillbox) (Game|GetPlayerCharacter 0) :!class /Script/Engine.PrimitiveComponent)
          (if true
            (if (Variables|/Game/Blob/Blueprint/BlobBP.BlobBP_C|GetIsAttacking _asblob_bp)
              (Actor|DestroyActor)
              (Variables|Default|SetAlive false)
              (Character|LaunchCharacter (Math|Vector|MakeVector (* (Math|Float|Sign(Float) (.yaw (Transformation|GetActorRotation))) 5e+01) 0.0 0.0) false false :!label _label)))))
      (:Out%201
        (if (not (Variables|/Game/Blob/Blueprint/BlobBP.BlobBP_C|GetIsHiding _asblob_bp))
          (if (Collision|IsOverlappingActor (Variables|Default|GetDetectionBox) (Game|GetPlayerCharacter 0) :!class /Script/Engine.PrimitiveComponent)
            (if (Variables|Default|GetAlive)
              (goto _label))))))
    (else
      (Variables|Default|SetSeconds 0.0)
      (Transformation|SetWorldRotation (Variables|Collision|GetCapsuleComponent) (Math|Rotator|MakeRotator 0.0 0.0 (+ (.Yaw (Math|Rotator|BreakRotator (Transformation|GetActorRotation))) 1.8e+02)) false false))))

(fn ConstructionScript)
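; Searching enemy that chases the player once they enter its detection area and hurts BlobBP on contact.
; On Tick, a looping MultiGate throttles a DetectionBox overlap check, which issues SimpleMoveToActor toward the player while the enemy is alive.
; A separate Box overlap launches the blob upward and horizontally along the hit normal's X axis, then applies damage through its DamageSystem.
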(event OnComponentBeginOverlap(Box)
  (params (OverlappedComponent :type Primitive%20Component%20Object%20Reference) (OtherActor :type Actor%20Object%20Reference) (OtherComp :type Primitive%20Component%20Object%20Reference) (OtherBodyIndex :type Integer) (bFromSweep :type Boolean) (SweepResult :type Hit%20Result%20Structure%20%28by%20ref%29))
  (bind _asblob_bp (Utilities|Casting|CastToBlobBP OtherActor))
  (Character|LaunchCharacter _asblob_bp (Math|Vector|MakeVector (* (.x (.Normal (Collision|BreakHitResult SweepResult))) -4.5e+02) 0.0 4e+02) true true)
  (Default|DamageSystem _asblob_bp (Variables|Default|GetDamage)))

(event EventTick
  (params (DeltaSeconds :type Float%20%28single-precision%29))
  (Utilities|FlowControl|MultiGate false true -1
    (:Out%201
      (if true
        (if (Collision|IsOverlappingActor (Variables|Default|GetDetectionBox) (Game|GetPlayerCharacter 0) :!class /Script/Engine.PrimitiveComponent)
          (if (Variables|Default|GetAlive)
            (AI|Navigation|SimpleMovetoActor 0 (Game|GetPlayerCharacter 0))))))))

(fn ConstructionScript)
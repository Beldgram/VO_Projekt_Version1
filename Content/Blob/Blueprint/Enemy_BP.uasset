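; Patrolling sprite enemy that damages and knocks back the player blob (BlobBP) on contact.
; The construction script builds a two-point InterpToMovement path from relative PointA and PointB, and a FlipFlop turns the sprite around at each reversal.
; Box overlap launches BlobBP upward and horizontally based on the sweep normal, then passes Damage to its DamageSystem.
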(event OnInterptoReverse(InterpToMovement)
  (params (ImpactResult :type Hit%20Result%20Structure%20%28by%20ref%29) (Time :type Float%20%28single-precision%29))
  (bind _papersprite (Variables|Default|GetPaperSprite))
  (Utilities|FlowControl|FlipFlop
    (:A
      (Transformation|SetWorldRotation _papersprite "0,180.000000, 0" false false))
    (:B
      (Transformation|SetWorldRotation _papersprite "0, 0, 0" false false))))

(event OnComponentBeginOverlap(Box)
  (params (OverlappedComponent :type Primitive%20Component%20Object%20Reference) (OtherActor :type Actor%20Object%20Reference) (OtherComp :type Primitive%20Component%20Object%20Reference) (OtherBodyIndex :type Integer) (bFromSweep :type Boolean) (SweepResult :type Hit%20Result%20Structure%20%28by%20ref%29))
  (bind _asblob_bp (Utilities|Casting|CastToBlobBP OtherActor))
  (Character|LaunchCharacter _asblob_bp (Math|Vector|MakeVector (* (.x (.Normal (Collision|BreakHitResult SweepResult))) -4.5e+02) 0.0 4e+02) true true)
  (Default|DamageSystem _asblob_bp (Variables|Default|GetDamage)))

(fn ConstructionScript
  (Variables|/Script/Engine.InterpToMovementComponent|SetControlPoints (Variables|Default|GetInterpToMovement) (Utilities|Array|MakeArray (Utilities|Struct|MakeInterpControlPoint (Variables|Default|GetPointA) true) (Utilities|Struct|MakeInterpControlPoint (Variables|Default|GetPointB) true))))
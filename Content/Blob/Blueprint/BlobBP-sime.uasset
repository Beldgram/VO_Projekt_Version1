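; Player-controlled 2D Blob character that runs, double-jumps, shoots and manages its own health, HUD and pause menu.
; A BlopState enum set by input, damage and landing selects the flipbook every Tick, with the Dead state also spawning the death screen.
; Each shot costs health and halts movement until shortly after release.
; Non-lethal damage knocks the blob back with input disabled until it lands and briefly sits.
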(event Custom|UpdateAnimation
  ;[1 1 1] Handle Animation
  (switch Utilities|FlowControl|Switch|SwitchonBlopState (Variables|Default|GetBlopState)
    (:NewEnumerator0
      (Sprite|SetFlipbook (Variables|Default|GetSprite) (select (> (Math|Vector|VectorLength (Transformation|GetVelocity)) 0.0) "/Game/Blob/Sprites/Character/Run.Run" "/Game/Blob/Sprites/Character/Stance.Stance")))
    (:NewEnumerator2
      (Sprite|SetFlipbook (Variables|Default|GetSprite) "/Game/Blob/Sprites/Character/Jump.Jump"))
    (:NewEnumerator4
      (Sprite|SetFlipbook (Variables|Default|GetSprite) "/Game/Blob/Sprites/Character/Hit.Hit"))
    (:NewEnumerator5
      (Sprite|SetFlipbook (Variables|Default|GetSprite) "/Game/Blob/Sprites/Character/Dead.Dead")
      (bind _returnvalue (UserInterface|CreateWidget "/Game/Blob/Blueprint/DeathScreen.DeathScreen_C"))
      (UserInterface|Viewport|AddtoViewport _returnvalue 0))
    (:NewEnumerator6
      (Sprite|SetFlipbook (Variables|Default|GetSprite) "/Game/Blob/Sprites/Character/Sitting.Sitting"))
    (:NewEnumerator7
      (Sprite|SetFlipbook (Variables|Default|GetSprite) "/Game/Blob/Sprites/Character/Shoot.Shoot"))))

(event Custom|Healing%20System
  (params (HealingIn :type Float%20%28single-precision%29))
  ;[1 1 1] Healing
  (if (>= (+ HealingIn (Variables|Default|GetHealthCurrent)) 1.0)
    (Variables|Default|SetHealthCurrent 1.0)
    (else
      (Variables|Default|SetHealthCurrent (+ HealingIn (Variables|Default|GetHealthCurrent)))))
  (CallFunction|UpdateAnimation))

(event Custom|Damage%20System
  (params (DamageIn :type Float%20%28single-precision%29))
  ;[1 1 1] Damage
  (Variables|Default|SetisHIt true)
  (Input|DisableInput (Game|GetPlayerController 0))
  (bind _output_get (Variables|Default|SetHealthCurrent (- (Variables|Default|GetHealthCurrent) DamageIn)))
  (if (<= _output_get 0.0)
    (Variables|Default|SetBlopState "NewEnumerator5")
    (else
      (Variables|Default|SetBlopState "NewEnumerator4")
      (Physics|AddForce (Variables|Character|GetCharacterMovement) (Math|Vector|MakeVector (* (Variables|Default|GetFacing) -5e+06) 0.0 1e+07)))))

(event EventTick
  (params (DeltaSeconds :type Float%20%28single-precision%29))
  ;[1 1 1] Tick - Updates animation
  (CallFunction|UpdateAnimation)
  (Math|Float|CompareFloat (.X (Math|Vector|BreakVector (Variables|/Script/Engine.MovementComponent|GetVelocity (Pawn|GetMovementComponent)))) 0.0
    (:>
      (Pawn|SetControlRotation (Pawn|GetController) (Math|Rotator|MakeRotator 0.0 0.0 0.0) :!label _label)
      (Variables|Default|SetFacing 1))
    (:==
      (if (Variables|Default|GetbisMovingRight)
        (goto _label)
        (else
          (Pawn|SetControlRotation (Pawn|GetController) (Math|Rotator|MakeRotator 0.0 0.0 1.8e+02) :!label _label_2)
          (Variables|Default|SetFacing -1))))
    (:<
      (goto _label_2))))

(event EventOnLanded
  (params (Hit :type Hit%20Result%20Structure%20%28by%20ref%29))
  ;[1 1 1] Handle Jump
  (Utilities|FlowControl|Sequence
    (:then_0
      (Utilities|FlowControl|DoN 2) ; enters at Reset
    )
    (:then_1
      (if (Utilities|Enum|NotEqual(Enum) (Variables|Default|GetBlopState) "NewEnumerator5")
        (if (Variables|Default|GetisHIt)
          (Variables|Default|SetBlopState "NewEnumerator6")
          (CallFunction|UpdateAnimation)
          (Utilities|FlowControl|Delay 0.5)
          (Variables|Default|SetBlopState "NewEnumerator0")
          (CallFunction|UpdateAnimation)
          (Variables|Default|SetisHIt false)
          (Input|EnableInput (Game|GetPlayerController 0))
          (else
            (Variables|Default|SetBlopState "NewEnumerator0")
            (CallFunction|UpdateAnimation)))))))

(event EventBeginPlay
  ;[1 1 1] Initialize
  (Utilities|FlowControl|Sequence
    (:then_0
      (Class|ActorComponent|SetIsReplicated (Variables|Default|GetSprite) true))
    (:then_1
      (bind _returnvalue (UserInterface|CreateWidget "/Game/Blob/Blueprint/Widget_HUD.Widget_HUD_C" (Game|GetPlayerController 0)))
      (bind _output_get (Variables|Default|SetHealthBar _returnvalue))
      (UserInterface|Viewport|AddtoViewport _output_get 0))))

(event Input|ActionEvents|InputActionPause
  (params (Key :type Key%20Structure))
  (bind _returnvalue (Game|GetPlayerController 0))
  ;[1 1 1] Pause
  (:Pressed
    (bind _returnvalue_2 (Game|GetCurrentLevelName true))
    (if (not (Utilities|Enum|Equal(Enum) _returnvalue_2 (Variables|Default|GetMenu_Level)))
      (if (not (Variables|Default|GetIsDeathScreenShown))
        (if (not (Variables|Default|GetIsPauseMenuShown))
          (bind _returnvalue_3 (UserInterface|CreateWidget "/Game/Blob/Blueprint/PauseMenu.PauseMenu_C"))
          (UserInterface|Viewport|AddtoViewport _returnvalue_3 0)
          (Variables|/Script/Engine.PlayerController|SetbShowMouseCursor _returnvalue true)
          (Input|SetInputModeGameandUI _returnvalue _returnvalue_3 "DoNotLock" true)
          (Variables|Default|SetIsPauseMenuShown true)
          (Game|SetGamePaused true))))))

(event Input|ActionEvents|InputActionJump
  (params (Key :type Key%20Structure))
  ;[1 1 1] Handle Jump
  (:Pressed
    (Utilities|FlowControl|DoN 2
      (:Exit
        (Character|Jump)
        (Variables|Default|SetBlopState "NewEnumerator2"))))
  (:Released
    (Character|StopJumping)))

(event Input|ActionEvents|InputActionShoot
  (params (Key :type Key%20Structure))
  ;[1 1 1] Shoot
  (:Pressed
    (if (> (Variables|Default|GetHealthCurrent) 0.05)
      (Variables|Default|SetHealthCurrent (- (Variables|Default|GetHealthCurrent) 0.05))
      (Variables|Default|SetcanMove false)
      (Game|SpawnActorfromClass "/Game/Blob/Blueprint/ShotBP.ShotBP_C" (Transformation|GetWorldTransform (Variables|Default|GetArrow1)) "AlwaysSpawn" 0 0)
      (Variables|Default|SetBlopState "NewEnumerator7")
      (Components|Movement|StopMovementImmediately (Variables|Character|GetCharacterMovement))
      (CallFunction|UpdateAnimation :!label _label)))
  (:Released
    (Utilities|FlowControl|RetriggerableDelay 0.5)
    (Variables|Default|SetBlopState "NewEnumerator0")
    (Variables|Default|SetcanMove true)
    (goto _label)))

(event Input|AxisEvents|InputAxisMoveRight
  (params (AxisValue :type Float%20%28single-precision%29))
  ;[1 1 1] Handle movement
  (if (Variables|Default|GetcanMove)
    (if (> AxisValue 0.0)
      (Variables|Default|SetbisMovingRight true)
      (elif (< AxisValue 0.0)
        (Variables|Default|SetbisMovingRight false)))
    (Pawn|Input|AddMovementInput "1.000000, 0, 0" AxisValue false)))

(fn ConstructionScript)
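; DestructableBlock3 is a Paper2D block that breaks after being hit by a set number of shots.
; When a ShotBP overlaps its Box, a DoN node capped at MaxNumHits counts the hit, then hides that shot and disables its collision.
; On the final hit, the block's sprite is hidden and loses collision rather than the actor being destroyed, and later shots are ignored.
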(event OnComponentBeginOverlap(Box)
  (params (OverlappedComponent :type Primitive%20Component%20Object%20Reference) (OtherActor :type Actor%20Object%20Reference) (OtherComp :type Primitive%20Component%20Object%20Reference) (OtherBodyIndex :type Integer) (bFromSweep :type Boolean) (SweepResult :type Hit%20Result%20Structure%20%28by%20ref%29))
  (bind _maxnumhits (Variables|Default|GetmaxNumHits))
  (bind _asshot_bp (Utilities|Casting|CastToShotBP OtherActor))
  (bind _counter (Utilities|FlowControl|DoN _maxnumhits)
    (:Exit
      (Development|SetHiddeninGame (Variables|/Game/Blob/Blueprint/ShotBP.ShotBP_C|GetShoot _asshot_bp) true false)
      (Collision|SetCollisionEnabled (Variables|/Game/Blob/Blueprint/ShotBP.ShotBP_C|GetBox _asshot_bp) "NoCollision")
      (if (== _counter _maxnumhits)
        (Development|SetHiddeninGame (Variables|Default|GetPaperSprite) true false)
        (Collision|SetCollisionEnabled (Variables|Default|GetPaperSprite) "NoCollision")))))

(event EventBeginPlay)

(event Collision|EventActorBeginOverlap
  (params (OtherActor :type Actor%20Object%20Reference)))

(event EventTick
  (params (DeltaSeconds :type Float%20%28single-precision%29)))

(fn ConstructionScript)